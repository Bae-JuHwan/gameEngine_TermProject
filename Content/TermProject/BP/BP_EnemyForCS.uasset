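; BP_EnemyForCS is a Barghest enemy that loops a bite animation until killed, with no movement or attack damage in this graph.
; BeginPlay starts the self-recalling, delayed Bite loop and hands a self reference to its 3D HP widget.
; Incoming damage goes to the BPHP component, whose events play a hurt sound or trigger the death roar, animation and delayed destruction.
; An IsDead flag stops biting and further damage.
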(event OnDamaged(BP_HP)
  (Audio|PlaySound2D "/Game/EffortVocalizations/cues/33_RAFE_-_Attack_C_Cue.33_RAFE_-_Attack_C_Cue" 1.0 1.0 0.0 0 0))

(event OnDeath(BP_HP)
  (Variables|Default|SetIsDead true)
  (Audio|PlaySound2D "/Game/MonsterRoarsAndGrowls/cues/02_Ferocious_Roar_Cue.02_Ferocious_Roar_Cue" 1.0 1.0 0.0 0 0)
  (Components|Animation|PlayAnimation (Variables|Character|GetMesh) "/Game/TermProject/Character/Enemy/BARGHEST_deathAggressive.BARGHEST_deathAggressive" false)
  (Utilities|FlowControl|Delay 1.5)
  (Actor|DestroyActor))

(event Custom|Bite
  (if (not (Variables|Default|GetIsDead))
    (Components|Animation|PlayAnimation (Variables|Character|GetMesh) "/Game/TermProject/Character/Enemy/BARGHEST_biteAggressive.BARGHEST_biteAggressive" false)
    (Utilities|FlowControl|Delay 2.0)
    (CallFunction|Bite)))

(event Collision|EventActorBeginOverlap
  (params (OtherActor :type Actor%20Object%20Reference)))

(event EventTick
  (params (DeltaSeconds :type Float%20%28single-precision%29)))

(event Game|Damage|EventAnyDamage
  (params (Damage :type Float%20%28single-precision%29) (DamageType :type Damage%20Type%20Object%20Reference) (InstigatedBy :type Controller%20Object%20Reference) (DamageCauser :type Actor%20Object%20Reference))
  (if (not (Variables|Default|GetIsDead))
    (Default|TakeDamage (Variables|Default|GetBP_HP) Damage)))

(event EventBeginPlay
  (CallFunction|Bite)
  (Variables|Default|SetBP_HP (Variables|Default|GetBP_HP))
  (bind _ascshpwidget (Utilities|Casting|CastToCSHPWidget (UserInterface|GetWidget (Variables|Default|Get3D%20Widget))))
  (Variables|/Game/TermProject/UMG/CSHPWidget.CSHPWidget_C|SetEnemyForCS _ascshpwidget self))

(fn ConstructionScript)