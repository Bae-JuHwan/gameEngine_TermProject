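; Dragon enemy character that damages what is in front of it and becomes the player's flying mount when killed.
; Tick uses a Delay to throttle three arrow-based line traces that apply damage roughly every two seconds.
; Incoming damage feeds the BP_HP component, which triggers roars and death, with health shown on a 3D widget.
; Death plays a montage, then attaches the dragon to Remy and switches the player to a seated, flying state.
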(event OnDamaged(BP_HP)
  (Audio|PlaySound2D "/Game/MonsterRoarsAndGrowls/wav/02_Ferocious_Roar.02_Ferocious_Roar" 1.0 1.0 0.0 0 0))

(event OnDeath(BP_HP)
  (bind _3d_widget (Variables|Default|Get3D%20Widget))
  (Variables|Default|SetDie true)
  (Variables|Default|SetIsDead true)
  (Audio|PlaySound2D "/Game/MonsterRoarsAndGrowls/wav/06_Battle_Roar.06_Battle_Roar" 1.0 1.0 0.0 0 0)
  (Animation|PlayAnimMontage "/Game/TermProject/AnimationMontage/DragonDeathMontage.DragonDeathMontage" 1.0 "Death")
  (Collision|SetCollisionEnabled (Variables|Character|GetMesh) "NoCollision")
  (Utilities|FlowControl|Delay 3.0)
  (bind _asremy (Utilities|Casting|CastToRemy (Game|Player|GetPlayerPawn 0)))
  (Components|SkeletalMesh|SetAnimInstanceClass (Variables|/Script/Engine.Character|GetMesh _asremy) "/Game/TermProject/AnimationMontage/RemySittingBP.RemySittingBP_C")
  (Transformation|AttachActorToActor self _asremy "DragonSocket" "SnapToTarget" "SnapToTarget" "SnapToTarget" true)
  (Transformation|SetRelativeLocation (Variables|Character|GetMesh) "-50.000000,0.000000,-450.000000" false false)
  (Variables|/Script/Engine.Pawn|SetbUseControllerRotationPitch _asremy true)
  (Variables|/Script/Engine.Pawn|SetbUseControllerRotationYaw _asremy true)
  (Variables|/Script/Engine.CharacterMovementComponent|SetbOrientRotationToMovement (Variables|/Script/Engine.Character|GetCharacterMovement _asremy) false)
  (Pawn|Components|CharacterMovement|SetMovementMode (Variables|/Script/Engine.Character|GetCharacterMovement _asremy) "MOVE_Flying" 0)
  (Variables|/Game/TermProject/BP/Remy.Remy_C|SetRideDragon? _asremy true)
  (UserInterface|SetWidget _3d_widget 0)
  (Rendering|SetVisibility _3d_widget false false))

(event EventBeginPlay
  (Variables|Default|SetBP_HP (Variables|Default|GetBP_HP))
  (bind _asdragon_hpwidget (Utilities|Casting|CastToDragonHPWidget (UserInterface|GetWidget (Variables|Default|Get3D%20Widget))))
  (Variables|/Game/TermProject/UMG/DragonHPWidget.DragonHPWidget_C|SetDragon _asdragon_hpwidget self))

(event Collision|EventActorBeginOverlap
  (params (OtherActor :type Actor%20Object%20Reference)))

(event EventTick
  (params (DeltaSeconds :type Float%20%28single-precision%29))
  (Utilities|FlowControl|Delay 2.0)
  (CallFunction|LineTrace)
  (CallFunction|LineTrace1)
  (CallFunction|LineTrace2))

(event Game|Damage|EventAnyDamage
  (params (Damage :type Float%20%28single-precision%29) (DamageType :type Damage%20Type%20Object%20Reference) (InstigatedBy :type Controller%20Object%20Reference) (DamageCauser :type Actor%20Object%20Reference))
  (if (not (Variables|Default|GetIsDead))
    (Default|TakeDamage (Variables|Default|GetBP_HP) Damage)))

(fn ConstructionScript)

(fn LineTrace
  (bind _arrow1 (Variables|Default|GetArrow1))
  (bind _returnvalue (Transformation|GetWorldLocation _arrow1))
  (bind _outhit (Collision|LineTraceByChannel _returnvalue (+ _returnvalue (* (Math|Vector|GetForwardVector _arrow1) 4e+02)) "TraceTypeQuery1" false 0 "None"))
  (Game|Damage|ApplyDamage (.hitactor _outhit) 1e+01 0 0))

(fn LineTrace1
  (bind _arrow2 (Variables|Default|GetArrow2))
  (bind _returnvalue (Transformation|GetWorldLocation _arrow2))
  (bind _outhit (Collision|LineTraceByChannel _returnvalue (+ _returnvalue (* (Math|Vector|GetForwardVector _arrow2) 4e+02)) "TraceTypeQuery1" false 0 "None"))
  (Game|Damage|ApplyDamage (.hitactor _outhit) 1e+01 0 0))

(fn LineTrace2
  (bind _arrow3 (Variables|Default|GetArrow3))
  (bind _returnvalue (Transformation|GetWorldLocation _arrow3))
  (bind _outhit (Collision|LineTraceByChannel _returnvalue (+ _returnvalue (* (Math|Vector|GetForwardVector _arrow3) 5e+02)) "TraceTypeQuery1" false 0 "None"))
  (Game|Damage|ApplyDamage (.hitactor _outhit) 1e+01 0 0))