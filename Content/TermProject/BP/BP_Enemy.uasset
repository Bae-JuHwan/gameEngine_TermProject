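; BP_Enemy is an enemy character that bites actors entering its sphere, takes damage and dies.
; A sphere overlap plays the bite montage and applies damage on completion, without rechecking range or death state.
; The BP_HP component receives damage and fires events for the hurt sound and the death roar, montage and delayed destroy.
; It also passes itself to its 3D health widget and updates horizontal Speed every tick.
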(event OnDamaged(BP_HP)
  ;[0.15 0.15 0.15 0.5] Damaged
  (Audio|PlaySound2D "/Game/EffortVocalizations/cues/33_RAFE_-_Attack_C_Cue.33_RAFE_-_Attack_C_Cue" 1.0 1.0 0.0 0 0))

(event OnDeath(BP_HP)
  ;[0.15 0.15 0.15 0.5] Damaged
  (Variables|Default|SetIsDead true)
  (Audio|PlaySound2D "/Game/MonsterRoarsAndGrowls/wav/02_Ferocious_Roar.02_Ferocious_Roar" 1.0 1.0 0.0 0 0)
  (Animation|PlayAnimMontage "/Game/TermProject/AnimationMontage/EnemyDeathMontage.EnemyDeathMontage" 1.0 "Death")
  (Utilities|FlowControl|Delay 1.0)
  (Actor|DestroyActor))

(event OnComponentBeginOverlap(Sphere)
  (params (OverlappedComponent :type Primitive%20Component%20Object%20Reference) (OtherActor :type Actor%20Object%20Reference) (OtherComp :type Primitive%20Component%20Object%20Reference) (OtherBodyIndex :type Integer) (bFromSweep :type Boolean) (SweepResult :type Hit%20Result%20Structure%20%28by%20ref%29))
  (if (!= OtherActor self)
    (Animation|Montage|PlayMontage (Variables|Character|GetMesh) "/Game/TermProject/AnimationMontage/EnemyBiteMontage.EnemyBiteMontage" 1.0 0.0 "Bite"
      (:OnCompleted
        (Game|Damage|ApplyDamage OtherActor 3.0 0 0)))))

(event EventBeginPlay
  (Variables|Default|SetBP_HP (Variables|Default|GetBP_HP))
  (bind _asenemy_hpwidget (Utilities|Casting|CastToEnemyHPWidget (UserInterface|GetWidget (Variables|Default|Get3D%20Widget))))
  (Variables|/Game/TermProject/UMG/EnemyHPWidget.EnemyHPWidget_C|SetEnemy _asenemy_hpwidget self))

(event Collision|EventActorBeginOverlap
  (params (OtherActor :type Actor%20Object%20Reference)))

(event EventTick
  (params (DeltaSeconds :type Float%20%28single-precision%29))
  (Variables|Default|SetSpeed (Math|Vector|VectorLengthXY (Transformation|GetVelocity))))

(event Game|Damage|EventAnyDamage
  (params (Damage :type Float%20%28single-precision%29) (DamageType :type Damage%20Type%20Object%20Reference) (InstigatedBy :type Controller%20Object%20Reference) (DamageCauser :type Actor%20Object%20Reference))
  ;[0.15 0.15 0.15 0.5] Damaged
  (if (not (Variables|Default|GetIsDead))
    (Default|TakeDamage (Variables|Default|GetBP_HP) Damage)
    (Utilities|FlowControl|Delay 0.2)))

(fn ConstructionScript)